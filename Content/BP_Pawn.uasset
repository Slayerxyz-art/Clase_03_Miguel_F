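; BP_Pawn is a test pawn that shuttles between two hard-coded world locations in an endless loop started on BeginPlay.
; Timed delays separate the moves, with only the second move using sweep, and a debug "Hello" prints during each cycle.
; Unconnected leftover nodes for rotating and offsetting the Cube component never run, and Tick and the construction script are empty.
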(event EventBeginPlay
  (Utilities|FlowControl|Delay 2.0 :!label _label)
  (Transformation|SetActorLocation "1347.000000,80.000000,260.000000" false false)
  (Utilities|FlowControl|Delay 2.0)
  (Development|PrintString "Hello")
  (Transformation|SetActorLocation "1247.000000,1050.000000,370.000000" true false)
  (Utilities|FlowControl|Delay 2.0)
  (Development|PrintString "Hello")
  (goto _label))

(event Collision|EventActorBeginOverlap
  (params (OtherActor :type Actor%20Object%20Reference)))

(event EventTick
  (params (DeltaSeconds :type Float%20%28single-precision%29)))

(fn ConstructionScript)